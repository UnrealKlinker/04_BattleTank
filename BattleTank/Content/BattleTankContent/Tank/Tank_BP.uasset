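; Player-controllable tank pawn Blueprint that wires components to their C++-exposed functions and maps input to camera, firing and driving.
; BeginPlay passes barrel, turret and tracks to the aiming and movement components, and reapplies meshes lost after C++ compiles plus track physical materials.
; Aim axes rotate an azimuth gimbal and spring arm, and Fire triggers the cannon.
; Driving supports both direct per-track throttle and intent-based move/turn through TankMovement.
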(event EventBeginPlay
  (bind _tankbarrel (Variables|Default|GetTankBarrel))
  (bind _left_tanktrack (Variables|Default|GetLeft%20TankTrack))
  (bind _right_tanktrack (Variables|Default|GetRight%20TankTrack))
  (Class|Tank|SetBarrelReference _tankbarrel)
  (Class|TankAimingComponent|Initialize (Variables|Default|GetTankAiming) _tankbarrel (Variables|Default|GetTankTurret))
  ;[1 1 1] Setting static meshes because they disappear after a C++ complile
  (Components|StaticMesh|SetStaticMesh (Variables|Default|GetTankTurret) "/Game/BattleTankContent/Tank/tank_fbx_Turret.tank_fbx_Turret")
  (Components|StaticMesh|SetStaticMesh _left_tanktrack "/Game/BattleTankContent/Tank/tank_fbx_Track.tank_fbx_Track")
  (Components|StaticMesh|SetStaticMesh _right_tanktrack "/Game/BattleTankContent/Tank/tank_fbx_Track.tank_fbx_Track")
  (Class|PrimitiveComponent|SetPhysMaterialOverride _left_tanktrack "/Game/BattleTankContent/Tank/TrackMaterial.TrackMaterial")
  (Class|PrimitiveComponent|SetPhysMaterialOverride _right_tanktrack "/Game/BattleTankContent/Tank/TrackMaterial.TrackMaterial")
  (Class|TankMovementComponent|Initialize (Variables|Default|GetTankMovement) _left_tanktrack _right_tanktrack))

(event Input|ActionEvents|InputActionFire
  (params (Key :type Key%20Structure))
  ;[1 1 1] Fire cannon
  (:Pressed
    (Class|Tank|Fire)))

(event Input|AxisEvents|InputAxisAimAzimuth
  (params (AxisValue :type Float%20%28single-precision%29))
  ;[1 1 1] Camera input binding
  (Transformation|AddLocalRotation (Variables|Default|GetAzimuth%20Gimbal) (Math|Rotator|MakeRotator 0.0 0.0 (* AxisValue 2.0)) false false))

(event Input|AxisEvents|InputAxisAimElevation
  (params (AxisValue :type Float%20%28single-precision%29))
  ;[1 1 1] Camera input binding
  (Transformation|AddLocalRotation (Variables|Default|GetSpringArm) (Math|Rotator|MakeRotator 0.0 AxisValue 0.0) false false))

(event Input|AxisEvents|InputAxisLeftTrackThrottle
  (params (AxisValue :type Float%20%28single-precision%29))
  ;[1 1 1] Throttle control functions through movement input binding
  (Class|TankTrack|SetThrottle (Variables|Default|GetLeft%20TankTrack) AxisValue))

(event Input|AxisEvents|InputAxisRightTrackThrottle
  (params (AxisValue :type Float%20%28single-precision%29))
  ;[1 1 1] Throttle control functions through movement input binding
  (Class|TankTrack|SetThrottle (Variables|Default|GetRight%20TankTrack) AxisValue))

(event Input|AxisEvents|InputAxisMoveForward
  (params (AxisValue :type Float%20%28single-precision%29))
  ;[1 1 1] Movement Inputs
  (Class|TankMovementComponent|IntendMoveForward (Variables|Default|GetTankMovement) AxisValue))

(event Input|AxisEvents|InputAxisTurnRight
  (params (AxisValue :type Float%20%28single-precision%29))
  ;[1 1 1] Movement Inputs
  (Class|TankMovementComponent|IntendTurnRight (Variables|Default|GetTankMovement) AxisValue))

(event Input|AxisEvents|InputAxisTurnLeft
  (params (AxisValue :type Float%20%28single-precision%29))
  ;[1 1 1] Movement Inputs
  (Class|TankMovementComponent|IntendTurnLeft (Variables|Default|GetTankMovement) AxisValue))

(fn ConstructionScript)